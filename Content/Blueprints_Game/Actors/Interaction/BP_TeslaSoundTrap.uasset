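; BP_TeslaSoundTrap is an interactable trap that plays a caught sound when a player walks into it while armed.
; Interact arms it and shows the Electricity and Sphere components.
; When a BP_PlayerBase overlaps the Box, it relays the sound through server and multicast events at the trap's location, then disarms and hides both components until the next Interact.
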(event OnComponentBeginOverlap(Box)
  (params (OverlappedComponent :type Primitive%20Component%20Object%20Reference) (OtherActor :type Actor%20Object%20Reference) (OtherComp :type Primitive%20Component%20Object%20Reference) (OtherBodyIndex :type Integer) (bFromSweep :type Boolean) (SweepResult :type Hit%20Result%20Structure%20%28by%20ref%29))
  (if (Variables|Default|GetIsEnabled)
    (bind _asbp_player_base (Utilities|Casting|CastToBP_PlayerBase OtherActor))
    (Utilities|IsValid _asbp_player_base
      (:Is%20Valid
        (CallFunction|ServerPlaySound)
        (Variables|Default|SetIsEnabled false)
        (Rendering|SetVisibility (Variables|Default|GetElectricity) false false)
        (Rendering|SetVisibility (Variables|Default|GetSphere) false false)))))

(event Custom|Server_PlaySound
  (CallFunction|MulticastPlaySound))

(event Custom|Multicast_PlaySound
  (Audio|PlaySoundatLocation "/Game/Assets/Audio/SFX/caught_sound.caught_sound" (Transformation|GetActorLocation self) "0, 0, 0" 1.0 1.0 0.0 0 0 0 0))

(event EventInteract
  (params (PlayerRef :type BP%20Player%20Base%20Object%20Reference))
  (if (not (Variables|Default|GetIsEnabled))
    (Variables|Default|SetIsEnabled true)
    (Rendering|SetVisibility (Variables|Default|GetElectricity) true false)
    (Rendering|SetVisibility (Variables|Default|GetSphere) true false)))

(fn ConstructionScript)