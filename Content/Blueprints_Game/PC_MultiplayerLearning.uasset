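; Player controller for a multiplayer game that manages the local HUD, menus, input modes and key pickup reporting.
; BeginPlay creates collapsed pause, inventory, victory and lose menus, and shows the HUD via a client event.
; Pause and inventory toggles switch movement, look and cursor, while end-game events close them, fade and lock further toggling.
; Tick line-traces for interactable crosshair feedback, and AddKey forwards through a server event to the GameState.
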(event Custom|ToggleInventory
  (bind _returnvalue (Game|GetPlayerCharacter 0))
  (bind _self self)
  (bind _inventorymenuref (Variables|Default|GetInventoryMenuRef))
  (bind _charactermovement (Variables|/Script/Engine.Character|GetCharacterMovement _returnvalue))
  ;[1 1 1] Inventory Toggle
  (if (not (Variables|Default|GetIsEndGameMenuOpened))
    (if (not (Variables|Default|GetIsPauseMenuOpened))
      (if (Variables|Default|GetIsInventoryOpened)
        (Variables|Default|SetIsInventoryOpened false)
        (CallFunction|FShowWidget "NewEnumerator0")
        (CallFunction|SetMovementMode _charactermovement)
        (Input|ResetIgnoreLookInput)
        (Variables|Default|SetbShowMouseCursor false)
        (Widget|SetVisibility _inventorymenuref "Collapsed")
        (Input|SetInputModeGameOnly _self false)
        (else
          (Variables|Default|SetIsInventoryOpened true)
          (CallFunction|FHideWidget "NewEnumerator0")
          (CallFunction|DisableMovement _charactermovement)
          (Input|SetIgnoreLookInput true)
          (Variables|Default|SetbShowMouseCursor true)
          (Widget|SetVisibility _inventorymenuref "SelfHitTestInvisible")
          (Input|SetInputModeGameandUI _self (Variables|Default|GetInventoryMenuRef) "DoNotLock" true false))))))

(event Custom|InitInventoryMenu
  ;[1 1 1] Init Inventory Menu (Client)
  (bind _returnvalue (UserInterface|CreateWidget "/Game/Blueprints_Game/UMG/Inventory/WB_InventoryMenu.WB_InventoryMenu_C"))
  (bind _output_get (Variables|Default|SetInventoryMenuRef _returnvalue))
  (Utilities|IsValid _output_get
    (:Is%20Valid
      (Widget|SetVisibility _output_get "Collapsed")
      (Utilities|IsValid (Variables|Default|GetInventoryMenuRef)
        (:Is%20Valid
          (UserInterface|Viewport|AddtoViewport (Variables|Default|GetInventoryMenuRef) 0))))))

(event Custom|InitLoseMenu
  ;[1 1 1] InitLoseMenu
  (bind _returnvalue (UserInterface|CreateWidget "/Game/Blueprints_Menu/Widgets/PauseMenu/WB_LoseMenu.WB_LoseMenu_C"))
  (bind _output_get (Variables|Default|SetLoseMenuRef _returnvalue))
  (Utilities|IsValid _output_get
    (:Is%20Valid
      (Widget|SetVisibility _output_get "Collapsed")
      (Utilities|IsValid (Variables|Default|GetLoseMenuRef)
        (:Is%20Valid
          (UserInterface|Viewport|AddtoViewport (Variables|Default|GetLoseMenuRef) 1))))))

(event Custom|EnableLoseMenu
  (bind _losemenuref (Variables|Default|GetLoseMenuRef))
  ;[1 1 1] EnableLoseMenu
  (CallFunction|FHandleEndGameMenu)
  (if (not (Variables|Default|GetIsEndGameMenuOpened))
    (Audio|PlaySoundatLocation "/Game/Assets/Audio/SFX/SC_Caught.SC_Caught" (Transformation|GetActorLocation (Game|Player|GetPlayerPawn 0)) "0, 0, 0" 1.0 1.0 0.0 0 0 0 0)
    (Default|FadeinLoseAnim (Variables|Default|GetWB_MainHud) 1.0 "Forward")
    (Utilities|FlowControl|Delay 1.0)
    (Widget|SetVisibility _losemenuref "Visible")
    (Input|SetInputModeGameandUI self _losemenuref "DoNotLock" true false)
    (Variables|Default|SetIsEndGameMenuOpened true)))

(event Custom|AddKey
  ;[1 1 1] AddKey
  (CallFunction|ServerAddKey))

(event Custom|Server_AddKey
  ;[1 1 1] AddKey
  (bind _asgs_multiplayer_learning (Utilities|Casting|CastToGS_MultiplayerLearning (Game|GetGameState)))
  (Default|ServerAddKey _asgs_multiplayer_learning))

(event Custom|InitPauseMenu
  ;[1 1 1] Init Pause Menu
  (bind _returnvalue (UserInterface|CreateWidget "/Game/Blueprints_Menu/Widgets/PauseMenu/WB_PauseMenu.WB_PauseMenu_C"))
  (bind _output_get (Variables|Default|SetPauseMenuRef _returnvalue))
  (Utilities|IsValid _output_get
    (:Is%20Valid
      (Widget|SetVisibility _output_get "Collapsed")
      (Utilities|IsValid (Variables|Default|GetPauseMenuRef)
        (:Is%20Valid
          (UserInterface|Viewport|AddtoViewport (Variables|Default|GetPauseMenuRef) 1))))))

(event Custom|ShowHideWidget
  (params (Show :type Boolean) (Widget :type E_GameWidgets%20Enum :default "NewEnumerator0"))
  ;[1 1 1] Init Main HUD (Client)
  (CallFunction|ClientShowHideWidget Show Widget))

(event Custom|Client_ShowHideWidget
  (params (Show :type Boolean) (Widget :type E_GameWidgets%20Enum :default "NewEnumerator0"))
  ;[1 1 1] Init Main HUD (Client)
  (if Show
    (CallFunction|FShowWidget Widget)
    (else
      (CallFunction|FHideWidget Widget))))

(event Custom|SetMovementMode
  (params (Target :type Character%20Movement%20Component%20Object%20Reference))
  ;[1 1 1] Inventory Toggle
  (Pawn|Components|CharacterMovement|SetMovementMode Target "MOVE_Walking" 0))

(event Custom|DisableMovement
  (params (Target :type Character%20Movement%20Component%20Object%20Reference))
  ;[1 1 1] Inventory Toggle
  (Pawn|Components|CharacterMovement|DisableMovement Target))

(event Custom|TogglePauseMenu
  (bind _returnvalue (Game|GetPlayerCharacter 0))
  (bind _self self)
  (bind _pausemenuref (Variables|Default|GetPauseMenuRef))
  (bind _charactermovement (Variables|/Script/Engine.Character|GetCharacterMovement _returnvalue))
  ;[1 1 1] Toggle Pause Menu
  (if (not (Variables|Default|GetIsEndGameMenuOpened))
    (if (Variables|Default|GetIsInventoryOpened)
      (CallFunction|ToggleInventory))
    (if (Variables|Default|GetIsPauseMenuOpened)
      (Variables|Default|SetIsPauseMenuOpened false)
      (CallFunction|SetMovementMode _charactermovement)
      (Input|ResetIgnoreLookInput)
      (Variables|Default|SetbShowMouseCursor false)
      (Widget|SetVisibility _pausemenuref "Hidden")
      (Input|SetInputModeGameOnly _self false)
      (else
        (Variables|Default|SetIsPauseMenuOpened true)
        (CallFunction|DisableMovement _charactermovement)
        (Input|SetIgnoreLookInput true)
        (Variables|Default|SetbShowMouseCursor true)
        (Widget|SetVisibility _pausemenuref "SelfHitTestInvisible")
        (Input|SetInputModeGameandUI _self (Variables|Default|GetPauseMenuRef) "DoNotLock" true false)))))

(event Custom|InitVictoryMenu
  ;[1 1 1] InitVictoryMenu
  (bind _returnvalue (UserInterface|CreateWidget "/Game/Blueprints_Menu/Widgets/PauseMenu/WB_VictoryMenu.WB_VictoryMenu_C"))
  (bind _output_get (Variables|Default|SetVictoryMenuRef _returnvalue))
  (Utilities|IsValid _output_get
    (:Is%20Valid
      (Widget|SetVisibility _output_get "Collapsed")
      (Utilities|IsValid (Variables|Default|GetVictoryMenuRef)
        (:Is%20Valid
          (UserInterface|Viewport|AddtoViewport (Variables|Default|GetVictoryMenuRef) 1))))))

(event Custom|EnableVictoryMenu
  (bind _victorymenuref (Variables|Default|GetVictoryMenuRef))
  ;[1 1 1] EnableVictoryMenu
  (CallFunction|FHandleEndGameMenu)
  (if (not (Variables|Default|GetIsEndGameMenuOpened))
    (Default|FadeinVictoryAnim (Variables|Default|GetWB_MainHud) 1.0 "Forward")
    (Utilities|FlowControl|Delay 1.0)
    (Widget|SetVisibility _victorymenuref "Visible")
    (Input|SetInputModeGameandUI self _victorymenuref "DoNotLock" true false)
    (Variables|Default|SetIsEndGameMenuOpened true)))

(event EventTick
  (params (DeltaSeconds :type Float%20%28single-precision%29))
  (bind _returnvalue (Game|GetPlayerCharacter 0))
  (bind _wb_mainhud (Variables|Default|GetWB_MainHud))
  (bind _asbp_player_base (Utilities|Casting|CastToBP_PlayerBase _returnvalue))
  ;[1 1 1] CrosshairChange
  (Utilities|IsValid _asbp_player_base
    (:Is%20Valid
      (bind _hitactor (Default|FLineTrace _asbp_player_base 3.5e+02 "None"))
      (Utilities|IsValid _wb_mainhud
        (:Is%20Valid
          (if (and (Utilities|IsValid _hitactor) (Utilities|DoesObjectImplementInterface _hitactor "/Game/Blueprints_Game/Interfaces/I_Interaction.I_Interaction_C"))
            (Default|ChangetoInteractCrosshair _wb_mainhud)
            (else
              (Default|ChangetoCrosshair _wb_mainhud))))))))

(event EventBeginPlay
  ;[1 1 1] Begin Play
  (CallFunction|SetMovementMode (Variables|/Script/Engine.Character|GetCharacterMovement (Game|GetPlayerCharacter 0)))
  (Input|ResetIgnoreLookInput)
  (Variables|Default|SetbShowMouseCursor false)
  (Input|SetInputModeGameOnly self false)
  (CallFunction|ShowHideWidget true "NewEnumerator0")
  (CallFunction|InitPauseMenu)
  (CallFunction|InitVictoryMenu)
  (CallFunction|InitLoseMenu)
  (CallFunction|InitInventoryMenu)
  (bind _gamemode (Class|IGameMode|GetGameModeRef(Message) (Game|GetGameMode)))
  (Variables|Default|SetGameMode _gamemode))

(fn ConstructionScript)

(fn FShowWidget
  (params (Widget :type E_GameWidgets%20Enum :default "NewEnumerator0"))
  (switch Utilities|FlowControl|Switch|SwitchonE_GameWidgets Widget
    (:NewEnumerator0
      (Variables|Default|GetWB_MainHud
        (:then
          _)
        (:else
          (bind _returnvalue (UserInterface|CreateWidget "/Game/Blueprints_Game/UMG/WB_MainHud.WB_MainHud_C"))
          (bind _output_get (Variables|Default|SetWB_MainHud _returnvalue))))
      (UserInterface|Viewport|AddtoViewport _output_get 0))))

(fn FHideWidget
  (params (Widget :type E_GameWidgets%20Enum :default "NewEnumerator0"))
  (switch Utilities|FlowControl|Switch|SwitchonE_GameWidgets Widget
    (:NewEnumerator0
      (bind _wb_mainhud (Variables|Default|GetWB_MainHud)
        (:then
          (Widget|RemovefromParent _wb_mainhud))
        (:else)))))

(fn FHandleEndGameMenu
  (if (Variables|Default|GetIsInventoryOpened)
    (CallFunction|ToggleInventory))
  (if (Variables|Default|GetIsPauseMenuOpened)
    (CallFunction|TogglePauseMenu))
  (CallFunction|DisableMovement (Variables|/Script/Engine.Character|GetCharacterMovement (Game|GetPlayerCharacter 0)))
  (Input|SetIgnoreLookInput true)
  (Variables|Default|SetbShowMouseCursor true))

(fn GetPlayerControllerRef
  (return self))