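; Enemy character that hunts players by sight and hearing and triggers the player's game loss when its capsule hits one.
; Perception updates pick the nearest sensed player, preferring sight over hearing, and pass it to AI_Controller as SeenPlayer.
; Target updates write the sensed state to the HasSeenPlayer? Blackboard key.
; A delay loop repeats a breathing sound at its location; FollowPlayer, called from an OnRep, is an empty stub.
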(event OnComponentHit(CapsuleComponent)
  (params (HitComponent :type Primitive%20Component%20Object%20Reference) (OtherActor :type Actor%20Object%20Reference) (OtherComp :type Primitive%20Component%20Object%20Reference) (NormalImpulse :type Vector :default "0, 0, 0") (Hit :type Hit%20Result%20Structure%20%28by%20ref%29))
  (bind _asbp_player_base (Utilities|Casting|CastToBP_PlayerBase OtherActor))
  (Utilities|IsValid _asbp_player_base
    (:Is%20Valid
      (Default|TriggerGameLose _asbp_player_base))))

(event OnPerceptionUpdated(AIPerception)
  (params (UpdatedActors :type Array%20of%20Actor%20Object%20References))
  (bind _aiperception (Variables|Default|GetAIPerception))
  (bind _outactors (Class|AIPerceptionComponent|GetCurrentlyPerceivedActors _aiperception "/Script/AIModule.AISense_Sight"))
  (Variables|Default|SetShortestDistance 5e+07)
  (if (Utilities|Array|IsNotEmpty _outactors)
    (Variables|Default|SetDetectedActors _outactors)
    (else
      (Variables|Default|SetDetectedActors (Class|AIPerceptionComponent|GetCurrentlyPerceivedActors (Variables|Default|GetAIPerception) "/Script/AIModule.AISense_Hearing"))))
  (for _array_element (Variables|Default|GetDetectedActors)
    (bind _asbp_player_base (Utilities|Casting|CastToBP_PlayerBase _array_element))
    (if (< (Transformation|GetDistanceTo _asbp_player_base) (Variables|Default|GetShortestDistance))
      (Variables|Default|SetShortestDistance (Transformation|GetDistanceTo _asbp_player_base))
      (Variables|Default|SetPawnToFollow _asbp_player_base)))
  (bind _asai_controller (Utilities|Casting|CastToAI_Controller (AI|GetAIController self)))
  (Variables|/Game/Blueprints_Game/Enemy/AI/AI_Controller.AI_Controller_C|SetSeenPlayer _asai_controller (Variables|Default|GetPawnToFollow)))

(event OnTargetPerceptionUpdated(AIPerception)
  (params (Actor :type Actor%20Object%20Reference) (Stimulus :type AI%20Stimulus%20Structure))
  (Utilities|Casting|CastToBP_PlayerBase Actor)
  (AI|Components|Blackboard|SetValueasBool (AI|GetBlackboard (AI|GetAIController self)) (Utilities|Name|MakeLiteralName "HasSeenPlayer?") (.bSuccessfullySensed (Utilities|Struct|BreakAIStimulus Stimulus))))

(event Custom|FollowPlayer)

(event EventBeginPlay
  (Utilities|FlowControl|Delay 2.0 :!label _label)
  (Audio|PlaySoundatLocation "/Game/Blueprints_Game/Enemy/Sounds/BreathingCue.BreathingCue" (Transformation|GetActorLocation self) "0, 0, 0" 1.0 1.0 0.0 0 0 0 0)
  (Utilities|FlowControl|Delay 1.0)
  (goto _label))

(event Collision|EventActorBeginOverlap
  (params (OtherActor :type Actor%20Object%20Reference)))

(fn ConstructionScript)

(fn OnRepIsSeeingPlayer
  (CallFunction|FollowPlayer))