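; Enemy character that chases pawns spotted by PawnSensing and supports montage-based turn-in-place.
; A sighting stores the pawn and sets IsSeeingPlayer, then starts AIMoveTo on authority; the flag's OnRep also calls FollowPlayer.
; TurnInPlace, not called within this graph, picks 90 or 180 degree turns from actor yaw when stationary and grounded.
; A timed Turning flag blocks overlapping turns, and Clear_TurnInPlace stops root-motion montages.
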(event OnSeePawn(PawnSensing)
  (params (Pawn :type Pawn%20Object%20Reference))
  (Variables|Default|SetPawnToFollow Pawn)
  (Variables|Default|SetIsSeeingPlayer true)
  (Networking|SwitchHasAuthority
    (:Authority
      (CallFunction|FollowPlayer))))

(event Custom|FollowPlayer
  (if (Variables|Default|GetIsSeeingPlayer)
    (AI|AIMoveTo self "0, 0, 0" (Variables|Default|GetPawnToFollow) 5.0 false)))

(event Custom|Play_Turn
  (params (MontageToPlay :type Anim%20Montage%20Object%20Reference) (PlayRate :type Float%20%28single-precision%29) (Duration :type Float%20%28single-precision%29))
  ;[1 1 1] Turnning Events
  (if (not (Variables|Default|GetTurning))
    (Variables|Default|SetTurning true)
    (Animation|Montage|PlayMontage (Variables|Character|GetMesh) MontageToPlay PlayRate
      (:then
        (Utilities|FlowControl|Delay Duration)
        (Variables|Default|SetTurning false)))))

(event Custom|Clear_Motion
  ;[1 1 1] Clear Root Motion
  (if (Class|Character|IsPlayingRootMotion)
    (Animation|StopAnimMontage (Animation|GetCurrentMontage :!class /Script/Engine.Character))))

(event Custom|Clear_TurnInPlace
  (params (Force :type Float%20%28double-precision%29))
  ;[1 1 1] Turnning Events
  (if (!= Force 0.0)
    (CallFunction|ClearMotion)))

(event Custom|Turn_Left_90
  ;[1 1 1] Turnning Events
  (CallFunction|PlayTurn 0 1.5 0.5))

(event Custom|Turn_Left_180
  ;[1 1 1] Turnning Events
  (CallFunction|PlayTurn 0 1.7 0.6))

(event Custom|Turn_Right_90
  ;[1 1 1] Turnning Events
  (CallFunction|PlayTurn 0 1.5 0.5))

(event Custom|Turn_Right_180
  ;[1 1 1] Turnning Events
  (CallFunction|PlayTurn 0 1.7 0.6))

(event EventBeginPlay)

(event Collision|EventActorBeginOverlap
  (params (OtherActor :type Actor%20Object%20Reference)))

(fn ConstructionScript)

(fn OnRepIsSeeingPlayer
  (CallFunction|FollowPlayer))

(fn TurninPlace
  (bind _returnvalue (Transformation|GetActorRotation))
  (bind _yaw (Math|Rotator|BreakRotator _returnvalue))
  (bind _returnvalue_2 (* _yaw 1.0))
  (if (and (not (AI|Components|NavMovement|IsFalling (Variables|Character|GetCharacterMovement))) (not (> (Math|Vector|VectorLengthXY (Variables|/Script/Engine.MovementComponent|GetVelocity (Variables|Character|GetCharacterMovement))) 0.0)))
    (if (or (> _returnvalue_2 45.0) (< _returnvalue_2 -45.0))
      (if (> _returnvalue_2 135.0)
        (CallFunction|TurnRight180)
        (elif (< _returnvalue_2 -135.0)
          (CallFunction|TurnLeft180)
          (elif (> _returnvalue_2 45.0)
            (CallFunction|TurnRight90)
            (elif (< _returnvalue_2 -45.0)
              (CallFunction|TurnLeft90))))))))