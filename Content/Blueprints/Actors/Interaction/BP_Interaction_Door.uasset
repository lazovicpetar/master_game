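; Interactable hinged door that toggles open and closed when a player interacts with it.
; Interact flips the RepNotify IsDoorClosed, which plays a timeline forward to open or reverses it to close.
; A dot product of the player-to-door direction and the door's forward vector picks a positive or negative 90-degree swing by player side.
; The timeline updates RepNotify DoorRotator, whose notify rotates the mesh.
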(event Custom|DoorRotatorNotify
  (Transformation|SetRelativeRotation (Variables|Default|GetStaticMesh1) (Variables|Default|GetDoorRotator) false false))

(event Custom|IsDoorClosedNotify
  (bind _self self)
  (if (not (Variables|Default|GetIsDoorClosed))
    (Variables|Default|SetDotProduct (Math|Vector|DotProduct (Math|Vector|Normalize (- (Transformation|GetActorLocation _self) (Transformation|GetActorLocation (Variables|Default|GetPlayer%20Ref)))) (Transformation|GetActorForwardVector _self)))
    (bind _alpha (Timeline|Timeline PlayFromStart)
      (:Update
        (Variables|Default|SetDoorRotator (Math|Rotator|MakeRotator 0.0 0.0 (Math|Float|Lerp 0.0 (Math|Float|SelectFloat 9e+01 -9e+01 (>= (Variables|Default|GetDotProduct) 0.0)) _alpha)))))
    (else
      (Timeline|Timeline Reverse))))

(event EventInteract
  (params (PlayerRef :type BP%20Player%20Base%20Object%20Reference))
  (Variables|Default|SetPlayer%20Ref PlayerRef)
  (if (Variables|Default|GetIsDoorClosed)
    (Variables|Default|SetIsDoorClosed false)
    (else
      (Variables|Default|SetIsDoorClosed true))))

(fn ConstructionScript
  (|CallParentFunction))

(fn OnRepIsDoorClosed
  (CallFunction|IsDoorClosedNotify))

(fn OnRepDoorRotator
  (CallFunction|DoorRotatorNotify))