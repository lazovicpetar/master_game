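; Master pickup actor that puts its item and amount into the interacting player's inventory.
; Interact calls a server event that runs AddItem on the player's BPCInventory component.
; On success, any remainder stays as the pickup's new amount, otherwise the actor is destroyed through a separate destroy event.
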(event Custom|ServerDestroyActor
  (Actor|DestroyActor))

(event Custom|ServerAddItem
  (params (Player%20Ref :type BP%20Player%20Base%20Object%20Reference))
  (Variables|Default|SetPlayer%20Ref Player%20Ref)
  (bind (_success _remainder) (Default|AddItem (Variables|/Game/Blueprints/Player/BP_PlayerBase.BP_PlayerBase_C|GetBPC_Inventory (Variables|Default|GetPlayer%20Ref)) (Variables|Default|GetItem) (Variables|Default|GetAmount)))
  (if _success
    (if (> _remainder 0)
      (Variables|Default|SetAmount _remainder)
      (else
        (CallFunction|ServerDestroyActor)))))

(event EventBeginPlay)

(event Collision|EventActorBeginOverlap
  (params (OtherActor :type Actor%20Object%20Reference)))

(event EventTick
  (params (DeltaSeconds :type Float%20%28single-precision%29)))

(event EventInteract
  (params (PlayerRef :type BP%20Player%20Base%20Object%20Reference))
  (CallFunction|ServerAddItem PlayerRef))

(fn ConstructionScript)