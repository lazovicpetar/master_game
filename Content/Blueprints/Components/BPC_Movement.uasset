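; Movement component that handles sprinting and crouching for an owning player character.
; Initialize stores the character reference and sets its walk speed as the starting max speed.
; Sprint events switch the CharacterMovement max walk speed between sprint and walk values through a shared setter, while crouch events call the character's built-in Crouch and UnCrouch.
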(event Custom|StartSprinting
  (CallFunction|SetMaxWalkSpeed (Variables|Default|GetSprintSpeed)))

(event Custom|StartCrouching
  (Character|Crouch (Variables|Default|GetPlayerRef)))

(event Custom|StopSprint
  (CallFunction|SetMaxWalkSpeed (Variables|Default|GetWalkSpeed)))

(event Custom|StopCrouching
  (Character|UnCrouch (Variables|Default|GetPlayerRef)))

(fn Initialize
  (params (Character :type Character%20Object%20Reference))
  (Variables|Default|SetPlayerRef Character)
  (Variables|/Script/Engine.CharacterMovementComponent|SetMaxWalkSpeed (Variables|/Script/Engine.Character|GetCharacterMovement (Variables|Default|GetPlayerRef)) (Variables|Default|GetWalkSpeed)))

(fn SetMaxWalkSpeed
  (params (MaxWalkSpeed :type Float%20%28double-precision%29))
  (Variables|/Script/Engine.CharacterMovementComponent|SetMaxWalkSpeed (Variables|/Script/Engine.Character|GetCharacterMovement (Variables|Default|GetPlayerRef)) MaxWalkSpeed))