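; Base networked first-person player character that handles movement, look, crouch, sprint, interaction and inventory toggling through Enhanced Input.
; Crouch and sprint update a stack-like MovementState array that drives BPCMovement, with remote calls mirrored to the server.
; Sprinting footsteps loop on a timer through server-to-multicast RPCs, and the server multicasts control rotation to the camera every tick.
; Interaction line-traces from the camera and calls I_Interaction targets on the server.
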(event Custom|Server_Crouch
  (params (IsCrouching :type Boolean))
  ;[1 1 1] Crouching
  (CallFunction|FCrouch IsCrouching))

(event Custom|Server_Sprint
  (params (IsSprinting :type Boolean))
  ;[1 1 1] Sprinting
  (CallFunction|FSprint IsSprinting))

(event Custom|ServerInteract
  (params (Target :type Object%20Object%20Reference) (PlayerRef :type BP%20Player%20Base%20Object%20Reference))
  ;[1 1 1] Interaction
  (Class|IInteraction|Interact(Message) Target PlayerRef))

(event Custom|Multicast_ReplicateRot
  (params (NewRotation :type Rotator))
  ;[1 1 1] Look
  (Networking|SwitchHasAuthority
    (:Authority
      _)
    (:Remote
      _))
  (Transformation|SetWorldRotation (Variables|Default|GetCamera) NewRotation false false))

(event Custom|Server_Initialize
  ;[1 1 1] Enable Input Mapping
  (CallFunction|FInitialize))

(event Custom|PlayFootstepsSFX
  ;[1 1 1] Movement
  (CallFunction|ServerPlayFootstepsSFX))

(event Custom|Server_PlayFootstepsSFX
  ;[1 1 1] Movement
  (CallFunction|MulticastPlayFootstepsSFX))

(event Custom|Multicast_PlayFootstepsSFX
  ;[1 1 1] Movement
  (Audio|PlaySoundatLocation "/Game/Assets/Audio/SFX/SC_Footsteps.SC_Footsteps" (Transformation|GetActorLocation) "0, 0, 0" 1.0 1.0 0.0 0 0 0 0))

(event Input|EnhancedActionEvents|EnhancedInputActionIA_Movement
  (params (ActionValue :type Vector%202D%20Structure) (ElapsedSeconds :type Float%20%28double-precision%29) (TriggeredSeconds :type Float%20%28double-precision%29) (InputAction :type Input%20Action%20Object%20Reference :default "/Game/Blueprints/Player/Input/IA_Movement.IA_Movement"))
  (bind _returnvalue (Transformation|GetVelocity))
  (bind _movementstate (Variables|Default|GetMovementState))
  ;[1 1 1] Movement
  (:Triggered
    (Pawn|Input|AddMovementInput (Transformation|GetActorForwardVector) (.x ActionValue) false)
    (Pawn|Input|AddMovementInput (Transformation|GetActorRightVector) (.y ActionValue) false)
    (if (Math|Boolean|ANDBoolean (Math|Boolean|ORBoolean (> (.x _returnvalue) 1e+02) (< (.x _returnvalue) -1e+02) (> (.y _returnvalue) 1e+02) (< (.y _returnvalue) -1e+02)) (not (AI|Components|NavMovement|IsFalling (Variables|Character|GetCharacterMovement))) (Utilities|Enum|Equal(Enum) (Utilities|Array|Get(acopy) _movementstate (Utilities|Array|LastIndex _movementstate)) (Variables|Default|GetSprintingState)))
      (if (not (Variables|Default|GetPlayingFootstepsSFX))
        (Variables|Default|SetPlayingFootstepsSFX true)
        (CallFunction|ServerPlayFootstepsSFX)
        (bind _returnvalue_2 (Utilities|Time|SetTimerbyEvent (delegate Custom|PlayFootstepsSFX) 0.35 true))
        (Variables|Default|SetFootstepsSFX_TH _returnvalue_2))
      (else
        (if (Utilities|Time|IsValidTimerHandle (Variables|Default|GetFootstepsSFX_TH)) :!label _label
          (Utilities|Time|ClearandInvalidateTimerbyHandle (Variables|Default|GetFootstepsSFX_TH))
          (Variables|Default|SetPlayingFootstepsSFX false)))))
  (:Completed
    (goto _label)))

(event Input|EnhancedActionEvents|EnhancedInputActionIA_Look
  (params (ActionValue :type Vector%202D%20Structure) (ElapsedSeconds :type Float%20%28double-precision%29) (TriggeredSeconds :type Float%20%28double-precision%29) (InputAction :type Input%20Action%20Object%20Reference :default "/Game/Blueprints/Player/Input/IA_Look.IA_Look"))
  ;[1 1 1] Look
  (Pawn|Input|AddControllerYawInput (.x ActionValue))
  (Pawn|Input|AddControllerPitchInput (.y ActionValue)))

(event Input|EnhancedActionEvents|EnhancedInputActionIA_Crouch
  (params (ActionValue :type Boolean) (ElapsedSeconds :type Float%20%28double-precision%29) (TriggeredSeconds :type Float%20%28double-precision%29) (InputAction :type Input%20Action%20Object%20Reference :default "/Game/Blueprints/Player/Input/IA_Crouch.IA_Crouch"))
  ;[1 1 1] Crouching
  (if ActionValue
    (CallFunction|FCrouch true)
    (else
      (CallFunction|FCrouch false))))

(event Input|EnhancedActionEvents|EnhancedInputActionIA_Sprint
  (params (ActionValue :type Boolean) (ElapsedSeconds :type Float%20%28double-precision%29) (TriggeredSeconds :type Float%20%28double-precision%29) (InputAction :type Input%20Action%20Object%20Reference :default "/Game/Blueprints/Player/Input/IA_Sprint.IA_Sprint"))
  ;[1 1 1] Sprinting
  (if ActionValue
    (CallFunction|FSprint true)
    (else
      (CallFunction|FSprint false))))

(event Input|EnhancedActionEvents|EnhancedInputActionIA_Action
  (params (ActionValue :type Boolean) (ElapsedSeconds :type Float%20%28double-precision%29) (TriggeredSeconds :type Float%20%28double-precision%29) (InputAction :type Input%20Action%20Object%20Reference :default "/Game/Blueprints/Player/Input/IA_Action.IA_Action"))
  ;[1 1 1] Interaction
  (:Started
    (bind _hitactor (CallFunction|FLineTrace 3e+02 "ForDuration"))
    (if (and (Utilities|IsValid _hitactor) (Utilities|DoesObjectImplementInterface _hitactor "/Game/Blueprints/Interfaces/I_Interaction.I_Interaction_C"))
      (CallFunction|ServerInteract _hitactor self))))

(event Input|EnhancedActionEvents|EnhancedInputActionIA_Inventory
  (params (ActionValue :type Boolean) (ElapsedSeconds :type Float%20%28double-precision%29) (TriggeredSeconds :type Float%20%28double-precision%29) (InputAction :type Input%20Action%20Object%20Reference :default "/Game/Blueprints/Player/Input/IA_Inventory.IA_Inventory"))
  ;[1 1 1] Inventory Toggle
  (:Started
    (bind _playercontroller (Class|IPlayerController|GetPlayerControllerRef(Message) (Game|GetPlayerController 0)))
    (Default|ToggleInventory _playercontroller)))

(event EventTick
  (params (DeltaSeconds :type Float%20%28single-precision%29))
  ;[1 1 1] Look
  (Networking|SwitchHasAuthority
    (:Authority
      (CallFunction|MulticastReplicateRot (Pawn|GetControlRotation :!class /Script/Engine.Pawn)))))

(event EventBeginPlay
  ;[1 1 1] Enable Input Mapping
  (bind _playercontroller (Class|IPlayerController|GetPlayerControllerRef(Message) (Pawn|GetController)))
  (Utilities|IsValid _playercontroller
    (:Is%20Valid
      (Input|AddMappingContext (PlayerController|LocalPlayerSubsystems|GetEnhancedInputLocalPlayerSubsystem _playercontroller) "/Game/Blueprints/Player/Input/IMC_Default.IMC_Default" 0 "(bIgnoreAllPressedKeysUntilRelease=True,bForceImmediately=False,bNotifyUserSettings=False)")
      (Components|SkinnedMesh|HideBonebyName (Variables|Character|GetMesh) "Head" "PBO_None")
      (CallFunction|FInitialize))))

(fn ConstructionScript)

(fn FCrouch
  (params (IsCrouching :type Boolean))
  (bind _movementstate (Variables|Default|GetMovementState))
  (bind _bpc_movement (Variables|Default|GetBPC_Movement))
  (bind _output_get (LocalVariables|SetIsCrouchingLocal IsCrouching))
  (Networking|SwitchHasAuthority
    (:Authority
      _)
    (:Remote
      (CallFunction|ServerCrouch _output_get)))
  (if (LocalVariables|GetIsCrouchingLocal)
    (Default|StartCrouching _bpc_movement)
    (Utilities|Array|SetArrayElem _movementstate (+ (Utilities|Array|LastIndex _movementstate) 1) "NewEnumerator1" true)
    (CallFunction|FSetMovementSpeed)
    (else
      (Default|StopCrouching _bpc_movement)
      (Utilities|Array|RemoveItem (Variables|Default|GetMovementState) "NewEnumerator1")
      (CallFunction|FSetMovementSpeed))))

(fn FSprint
  (params (IsSprinting :type Boolean))
  (bind _bpc_movement (Variables|Default|GetBPC_Movement))
  (bind _movementstate (Variables|Default|GetMovementState))
  (bind _output_get (LocalVariables|SetIsSprintingLocal IsSprinting))
  (Networking|SwitchHasAuthority
    (:Authority
      _)
    (:Remote
      (CallFunction|ServerSprint _output_get)))
  (if (LocalVariables|GetIsSprintingLocal)
    (Default|StartSprinting _bpc_movement)
    (Utilities|Array|SetArrayElem _movementstate (+ (Utilities|Array|LastIndex _movementstate) 1) "NewEnumerator2" true)
    (CallFunction|FSetMovementSpeed)
    (else
      (Default|StopSprint _bpc_movement)
      (Utilities|Array|RemoveItem (Variables|Default|GetMovementState) "NewEnumerator2")
      (CallFunction|FSetMovementSpeed))))

(fn FInitialize
  (Networking|SwitchHasAuthority
    (:Authority
      _)
    (:Remote
      (CallFunction|ServerInitialize)))
  (Default|Initialize (Variables|Default|GetBPC_Movement) self))

(fn FLineTrace
  (params (Length :type Float%20%28double-precision%29) (DebugType :type EDrawDebugTrace%20Enum :default "None"))
  (bind _camera (Variables|Default|GetCamera))
  (bind _returnvalue (Transformation|GetWorldLocation _camera))
  (bind _outhit (Collision|LineTraceByChannel _returnvalue (+ _returnvalue (* Length (Math|Vector|GetForwardVector _camera))) "TraceTypeQuery1" false 0 DebugType))
  (return (.HitActor (Collision|BreakHitResult _outhit))))

(fn FSetMovementSpeed
  (bind _movementstate (Variables|Default|GetMovementState))
  (bind _bpc_movement (Variables|Default|GetBPC_Movement))
  (switch Utilities|FlowControl|Switch|SwitchonE_MovementStates (Utilities|Array|Get(acopy) _movementstate (Utilities|Array|LastIndex _movementstate))
    (:NewEnumerator0
      (Default|StopCrouching _bpc_movement)
      (Variables|/Script/Engine.CharacterMovementComponent|SetMaxWalkSpeed (Variables|Character|GetCharacterMovement) (Variables|Default|GetWalkSpeed)))
    (:NewEnumerator1
      (Default|StartCrouching _bpc_movement))
    (:NewEnumerator2
      (Default|StopCrouching _bpc_movement)
      (Default|StartSprinting _bpc_movement))))

(fn GetPlayerRef
  (return self))