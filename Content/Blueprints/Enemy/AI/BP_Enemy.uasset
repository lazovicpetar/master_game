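; Enemy Blueprint that passes player perception results to its AI controller and Blackboard.
; When AI Perception updates on a BP_PlayerBase, it writes the sensed result to the "HasSeenPlayer?" key.
; It then sets SeenPlayer on AI_Controller to that player, even when sensing fails.
; An IsSeeingPlayer RepNotify calls FollowPlayer, which is empty, and nothing here sets that variable.
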(event OnTargetPerceptionUpdated(AIPerception)
  (params (Actor :type Actor%20Object%20Reference) (Stimulus :type AI%20Stimulus%20Structure))
  (bind _self self)
  (bind _returnvalue (AI|GetAIController _self))
  (bind _asbp_player_base (Utilities|Casting|CastToBP_PlayerBase Actor))
  (AI|Components|Blackboard|SetValueasBool (AI|GetBlackboard _returnvalue) (Utilities|Name|MakeLiteralName "HasSeenPlayer?") (.bSuccessfullySensed (Utilities|Struct|BreakAIStimulus Stimulus)))
  (bind _asai_controller (Utilities|Casting|CastToAI_Controller _returnvalue))
  (Variables|/Game/Blueprints/Enemy/AI/AI_Controller.AI_Controller_C|SetSeenPlayer _asai_controller _asbp_player_base))

(event Custom|FollowPlayer)

(event EventBeginPlay)

(event Collision|EventActorBeginOverlap
  (params (OtherActor :type Actor%20Object%20Reference)))

(event EventTick
  (params (DeltaSeconds :type Float%20%28single-precision%29)))

(fn ConstructionScript)

(fn OnRepIsSeeingPlayer
  (CallFunction|FollowPlayer))