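; Enemy pawn that chases pawns it spots through a PawnSensing component.
; Seeing a pawn stores it as the follow target and sets IsSeeingPlayer, then the authority calls FollowPlayer, which issues AI MoveTo toward that target.
; IsSeeingPlayer uses a RepNotify that also calls FollowPlayer, and nothing in this Blueprint clears the flag.
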(event OnSeePawn(PawnSensing)
  (params (Pawn :type Pawn%20Object%20Reference))
  (Variables|Default|SetPawnToFollow Pawn)
  (Variables|Default|SetIsSeeingPlayer true)
  (Networking|SwitchHasAuthority
    (:Authority
      (CallFunction|FollowPlayer))))

(event Custom|FollowPlayer
  (if (Variables|Default|GetIsSeeingPlayer)
    (AI|AIMoveTo self "0, 0, 0" (Variables|Default|GetPawnToFollow) 5.0 false)))

(event EventBeginPlay)

(event Collision|EventActorBeginOverlap
  (params (OtherActor :type Actor%20Object%20Reference)))

(event EventTick
  (params (DeltaSeconds :type Float%20%28single-precision%29)))

(fn ConstructionScript)

(fn OnRepIsSeeingPlayer
  (CallFunction|FollowPlayer))